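; BP_chair is a chair actor for VR with an unfinished sit interaction.
; Its Sit_detection_collision component sets the Değdi flag while a VRCharacter overlaps it, printing debug messages on enter and exit.
; The Oculus use button checks that flag but triggers nothing.
; The disconnected sit logic would offset the chair actor itself by OturmaNoktası (sitting point), with sweep and teleport, then print a confirmation.
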(event `self.sit_detection_collision.OnComponentBeginOverlap`
  (params (OverlappedComponent :type "PrimitiveComponent Object Reference") (OtherActor :type "Actor Object Reference") (OtherComp :type "PrimitiveComponent Object Reference") (OtherBodyIndex :type Integer) (bFromSweep :type Boolean) (SweepResult :type "HitResult Structure (by ref)"))
  (cast `/Game/project/VRCharacter` OtherActor)
  (set `self.değdi` true)
  (`KismetSystemLibrary.PrintString` "değdi"))

(event `self.sit_detection_collision.OnComponentEndOverlap`
  (params (OverlappedComponent :type "PrimitiveComponent Object Reference") (OtherActor :type "Actor Object Reference") (OtherComp :type "PrimitiveComponent Object Reference") (OtherBodyIndex :type Integer))
  (cast `/Game/project/VRCharacter` OtherActor)
  (set `self.değdi` false)
  (`KismetSystemLibrary.PrintString` "değmedi"))

(event `InputAction|OculusUseButton`
  (params (Key :type "Key Structure"))
  (:`Pressed`
    (if (`self.değdi`)
      _)))

(fn `UserConstructionScript`)